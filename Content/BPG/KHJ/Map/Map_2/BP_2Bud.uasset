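; BP_2Bud manages the Map_2 HUD, keeping its player list in sync with player name changes.
; On BeginPlay it creates the 2HudWidget, adds it to the viewport and switches to UI-only input with a visible cursor.
; BindPlayerState subscribes to a passed object's name-change dispatcher and triggers an immediate update.
; UpdatePlayerName refreshes the list, falling back to a self-retrying timer until the widget exists.
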(event EventBeginPlay
  (bind _returnvalue (Game|GetPlayerController 0))
  (bind _returnvalue_2 (UserInterface|CreateWidget "/Game/BPG/KHJ/Map/Map_2/2HudWidget.2HudWidget_C"))
  (bind _output_get (Variables|Default|Set2HudWidget _returnvalue_2))
  (UserInterface|Viewport|AddtoViewport _output_get 0)
  (Input|SetInputModeUIOnly _returnvalue 0 "DoNotLock")
  (Variables|/Script/Engine.PlayerController|SetbShowMouseCursor _returnvalue true))

(fn ConstructionScript)

(fn BindPlayerState
  (params (NewParam :type BP2%20Player%20State%20Object%20Reference))
  (EventDispatchers|BindEventtoNewEventDispatcherChangePlayerName NewParam (EventDispatchers|CreateEvent :!event UpdatePlayerName))
  (CallFunction|UpdatePlayerName))

(fn WaitCreateHudWidget
  (bind _2hudwidget (Variables|Default|Get2HudWidget))
  (Utilities|IsValid _2hudwidget
    (:Is%20Valid
      (Default|PlayerListUpdate _2hudwidget))
    (:Is%20Not%20Valid
      (Utilities|Time|SetTimerbyFunctionName 0 "WaitCreateHudWidget" 0.1))))

(fn UpdatePlayerName
  (params (PlayerName :type String))
  (bind _2hudwidget (Variables|Default|Get2HudWidget))
  (Utilities|IsValid _2hudwidget
    (:Is%20Valid
      (Default|PlayerListUpdate _2hudwidget))
    (:Is%20Not%20Valid
      (if (not (Class|KismetSystemLibrary|TimerExists 0 "WaitCreateHudWidget"))
        (Utilities|Time|SetTimerbyFunctionName 0 "WaitCreateHudWidget" 0.1)))))