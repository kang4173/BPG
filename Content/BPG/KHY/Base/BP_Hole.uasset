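; BP_Hole is a hole actor meant to drag nearby NewBlueprint_Khy actors horizontally toward its center.
; Sphere1 overlaps and a one-time Tick scan maintain the OverlappingActors array.
; Attract2 starts a looping timer on Active, which lerps each actor's XY via a timeline, preserving Z; Clear stops it.
; Debug prints, unconnected experiments and a separate BaseChar Attract function, uncalled here, suggest work in progress.
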(event OnComponentBeginOverlap(Sphere1)
  (params (OverlappedComponent :type Primitive%20Component%20Object%20Reference) (OtherActor :type Actor%20Object%20Reference) (OtherComp :type Primitive%20Component%20Object%20Reference) (OtherBodyIndex :type Integer) (bFromSweep :type Boolean) (SweepResult :type Hit%20Result%20Structure%20%28by%20ref%29))
  (bind _asnew_blueprint_khy (Utilities|Casting|CastToNewBlueprint_Khy OtherActor))
  (Utilities|Array|AddUnique (Variables|Default|GetOverlapping%20Actors) _asnew_blueprint_khy))

(event OnComponentEndOverlap(Sphere1)
  (params (OverlappedComponent :type Primitive%20Component%20Object%20Reference) (OtherActor :type Actor%20Object%20Reference) (OtherComp :type Primitive%20Component%20Object%20Reference) (OtherBodyIndex :type Integer))
  (bind _asnew_blueprint_khy (Utilities|Casting|CastToNewBlueprint_Khy OtherActor))
  (Utilities|Array|RemoveItem (Variables|Default|GetOverlapping%20Actors) _asnew_blueprint_khy))

(event Custom|Attract2
  (Utilities|Time|SetTimerbyFunctionName 0 "Active" 0.1 true))

(event Custom|CallArray
  (for _array_element (Variables|Default|GetOverlapping%20Actors)
    (Development|PrintString (Utilities|GetDisplayName _array_element) true true "(R=1.000000,G=0.000000,B=0.066279,A=1.000000)")))

(event Custom|Active
  (bind _returnvalue (Transformation|GetActorLocation))
  (bind (_x _y) (Math|Vector|BreakVector _returnvalue))
  (Development|PrintString "Hello")
  (for _array_element (Variables|Default|GetOverlapping%20Actors)
    (bind _curve (Timeline|타임라인_0 SetNewTime)
      (:Update
        (Development|PrintString (Utilities|String|ToString(Float) _curve) true true "(R=0.000000,G=0.874921,B=1.000000,A=1.000000)" 1e+01)
        (Transformation|SetActorLocation _array_element (Math|Interpolation|Ease "Linear" _curve (Math|Vector|MakeVector (.X (Math|Vector|BreakVector (Transformation|GetActorLocation _array_element))) (.Y (Math|Vector|BreakVector (Transformation|GetActorLocation _array_element))) (.Z (Math|Vector|BreakVector (Transformation|GetActorLocation _array_element)))) (Math|Vector|MakeVector _x _y (.Z (Math|Vector|BreakVector (Transformation|GetActorLocation _array_element))))) false false)))))

(event Custom|ResetTimeline
  (bind _returnvalue (Transformation|GetActorLocation))
  (bind (_x _y) (Math|Vector|BreakVector _returnvalue))
  (bind _curve (Timeline|타임라인_0 SetNewTime)
    (:Update
      (Development|PrintString (Utilities|String|ToString(Float) _curve) true true "(R=0.000000,G=0.874921,B=1.000000,A=1.000000)" 1e+01)
      (Transformation|SetActorLocation (stale Custom|Active _array_element) (Math|Interpolation|Ease "Linear" _curve (Math|Vector|MakeVector (.X (Math|Vector|BreakVector (Transformation|GetActorLocation (stale Custom|Active _array_element)))) (.Y (Math|Vector|BreakVector (Transformation|GetActorLocation (stale Custom|Active _array_element)))) (.Z (Math|Vector|BreakVector (Transformation|GetActorLocation (stale Custom|Active _array_element))))) (Math|Vector|MakeVector _x _y (.Z (Math|Vector|BreakVector (Transformation|GetActorLocation (stale Custom|Active _array_element)))))) false false))))

(event Custom|Clear
  (Utilities|Time|ClearTimerbyFunctionName 0 "Active"))

(event EventTick
  (params (DeltaSeconds :type Float%20%28single-precision%29))
  (Utilities|FlowControl|DoOnce false
    (:Completed
      (Utilities|IsValid (Utilities|Array|Get(acopy) (Collision|GetOverlappingActors (Variables|Default|GetSphere1) "/Game/BPG/KHY/Base/NewBlueprint_Khy.NewBlueprint_Khy_C" :!class /Script/Engine.PrimitiveComponent))
        (:Is%20Valid
          (for _array_element (Collision|GetOverlappingActors (Variables|Default|GetSphere1) "/Game/BPG/KHY/Base/NewBlueprint_Khy.NewBlueprint_Khy_C" :!class /Script/Engine.PrimitiveComponent)
            (Development|PrintString (Utilities|GetDisplayName _array_element) true true "(R=0.000000,G=0.000000,B=0.000000,A=1.000000)")
            (bind _asnew_blueprint_khy (Utilities|Casting|CastToNewBlueprint_Khy _array_element))
            (Utilities|Array|AddUnique (Variables|Default|GetOverlapping%20Actors) _asnew_blueprint_khy)))))))

(event EventBeginPlay)

(fn ConstructionScript)

(fn Attract
  (bind _returnvalue (Transformation|GetActorLocation))
  (bind (_x _y) (Math|Vector|BreakVector _returnvalue))
  (Development|PrintString "Hello" true true "(R=0.834476,G=0.000000,B=1.000000,A=1.000000)")
  (for (_array_element _array_index) (Collision|GetOverlappingActors (Variables|Default|GetSphere1) "/Script/BPG.BaseChar" :!class /Script/Engine.PrimitiveComponent)
    (Development|PrintString (Utilities|String|ToString(Integer) _array_index) true true "(R=1.000000,G=0.750000,B=0.000000,A=1.000000)")
    (bind _asbase_char (Utilities|Casting|CastToBaseChar _array_element))
    (Transformation|SetActorLocation _asbase_char (Math|Interpolation|Ease "Linear" (+ 0.0 (Utilities|Time|GetWorldDeltaSeconds)) (Math|Vector|MakeVector (.X (Math|Vector|BreakVector (Transformation|GetActorLocation _asbase_char))) (.Y (Math|Vector|BreakVector (Transformation|GetActorLocation _asbase_char))) (.Z (Math|Vector|BreakVector (Transformation|GetActorLocation _asbase_char)))) (Math|Vector|MakeVector _x _y (.Z (Math|Vector|BreakVector (Transformation|GetActorLocation _asbase_char))))) false false)))