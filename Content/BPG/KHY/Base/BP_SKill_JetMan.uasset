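; JetMan skill Blueprint that changes the character's movement into a gravity-free, high-acceleration mode while it is active.
; ComSetting runs the parent setup, then zeroes gravity on Char, raises max acceleration and enables strong separate braking friction for abrupt stops.
; EndPlay restores hardcoded movement values rather than saved ones, then moves the character 1000 units down without sweep.
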(event EventBeginPlay)

(event EventTick
  (params (DeltaSeconds :type Float%20%28single-precision%29)))

(event EventComSetting
  (bind _char (Variables|Default|GetChar))
  (bind _charactermovement (Variables|/Script/Engine.Character|GetCharacterMovement _char))
  (|CallParentFunction)
  (Variables|/Script/Engine.CharacterMovementComponent|SetGravityScale _charactermovement 0.0)
  (Variables|/Script/Engine.CharacterMovementComponent|SetMaxAcceleration _charactermovement 1.5e+04)
  (Variables|/Script/Engine.CharacterMovementComponent|SetbUseSeparateBrakingFriction _charactermovement true)
  (Variables|/Script/Engine.CharacterMovementComponent|SetBrakingFriction _charactermovement 1e+04))

(event EventEndPlay
  (params (EndPlayReason :type EEndPlayReason%20Enum :default "Destroyed"))
  (bind _char (Variables|Default|GetChar))
  (bind _char_2 (Variables|Default|GetChar))
  (bind _returnvalue (Transformation|GetActorLocation _char_2))
  (bind _charactermovement (Variables|/Script/Engine.Character|GetCharacterMovement _char))
  (bind (_x _y _z) (Math|Vector|BreakVector _returnvalue))
  (Variables|/Script/Engine.CharacterMovementComponent|SetGravityScale _charactermovement 1.0)
  (Variables|/Script/Engine.CharacterMovementComponent|SetMaxAcceleration _charactermovement 2048.0)
  (Variables|/Script/Engine.CharacterMovementComponent|SetBrakingFriction _charactermovement 0.0)
  (Variables|/Script/Engine.CharacterMovementComponent|SetbUseSeparateBrakingFriction _charactermovement false)
  (Transformation|SetActorLocation _char_2 (Math|Vector|MakeVector _x _y (- _z 1e+03)) false false))